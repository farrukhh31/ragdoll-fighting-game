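; BP_SharedCamera is a shared multiplayer camera that follows and frames all players with a spring arm.
; Each Tick, when more than one player is present, it moves to the average of valid pawn locations, dividing by the total player count.
; It then finds the farthest pawn from that center and maps that distance to a clamped multiplier on MinArmLength, zooming out as players spread apart.
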(event `self.ReceiveTick`
  (params (DeltaSeconds :type "Float (single-precision)"))
  ;[1 1 1] Set Camera Location
  (bind _returnvalue (`GameModeBase.GetNumPlayers` (`GameplayStatics.GetGameMode`)))
  (if (> _returnvalue 1)
    (set `self.locationSum` (0.0 0.0 0.0))
    (for _index (range _returnvalue)
      (bind _returnvalue_2 (`GameplayStatics.GetPlayerPawn` _index))
      (`/Engine/EditorBlueprintResources/StandardMacros.IsValid` _returnvalue_2
        (:`Is Valid`
          (set `self.locationSum` (+ (`self.locationSum`) (`self.K2_GetActorLocation` _returnvalue_2))))))
    (`self.K2_SetActorLocation` (/ (`self.locationSum`) _returnvalue))
    (set `self.maxDistFromCenterPoint` 0.0)
    (bind _returnvalue_3 (`GameModeBase.GetNumPlayers` (`GameplayStatics.GetGameMode`)))
    (if (> _returnvalue_3 1)
      (for _index_2 (range _returnvalue_3)
        (bind _returnvalue_4 (`GameplayStatics.GetPlayerPawn` _index_2))
        (`/Engine/EditorBlueprintResources/StandardMacros.IsValid` _returnvalue_4
          (:`Is Valid`
            (bind _returnvalue_5 (`KismetMathLibrary.Vector_Distance` (`self.K2_GetActorLocation`) (`self.K2_GetActorLocation` _returnvalue_4)))
            (if (> _returnvalue_5 (`self.maxDistFromCenterPoint`))
              (set `self.maxDistFromCenterPoint` _returnvalue_5)))))
      (set `SpringArmComponent.TargetArmLength` (* (`KismetMathLibrary.MapRangeClamped` (`self.maxDistFromCenterPoint`) 100.0 1200.0 1.0 3.0) (`self.minArmLength`)) (`self.SpringArm`))
      (else
        (set `SpringArmComponent.TargetArmLength` (`self.minArmLength`) (`self.SpringArm`))))))

(fn `UserConstructionScript`)